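; BP_LevelReset is a trigger actor that restarts the current level when the player pawn overlaps its Collision component.
; On BeginPlay it caches the current level name and starts a camera fade in from a solid dark blue.
; On player overlap it fades the camera to the same blue, waits for the fade to finish, then reopens the cached level by name.
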(event `self.Collision.OnComponentBeginOverlap`
  (params (OverlappedComponent :type "PrimitiveComponent Object Reference") (OtherActor :type "Actor Object Reference") (OtherComp :type "PrimitiveComponent Object Reference") (OtherBodyIndex :type Integer) (bFromSweep :type Boolean) (SweepResult :type "HitResult Structure (by ref)"))
  (if (== OtherActor (`GameplayStatics.GetPlayerPawn` 0))
    (`PlayerCameraManager.StartCameraFade` (`GameplayStatics.GetPlayerCameraManager` 0) 0.2 1.0 1.0 (struct :`R` 0.066929 :`G` 0.042502 :`B` 0.429167 :`A` 1.0) false false)
    (`KismetSystemLibrary.Delay` 1.0)
    (`GameplayStatics.OpenLevel` (`KismetStringLibrary.Conv_StringToName` (stale `self.ReceiveBeginPlay` _returnvalue)))))

(event `self.ReceiveBeginPlay`
  (`|ExecutionSequence`
    (:`then_0`
      (bind _returnvalue (`GameplayStatics.GetCurrentLevelName` true)))
    (:`then_1`
      (`PlayerCameraManager.StartCameraFade` (`GameplayStatics.GetPlayerCameraManager` 0) 1.0 0.0 1.0 (struct :`R` 0.066626 :`G` 0.042311 :`B` 0.423268 :`A` 1.0) false false))))

(fn `UserConstructionScript`)